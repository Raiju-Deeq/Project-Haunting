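; BP_Eye2 is an actor that probes a cone-like region ahead of itself with debug-drawn sphere traces, apparently as a vision prototype.
; Each tick, a loop doubles the sphere diameter and steps forward along the actor's facing by the new radius, producing overlapping, growing spheres.
; Each zero-length trace uses the Visibility channel, but its hit results are unused.
; The working location and diameter reset after the loop.
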(event EventTick
  (params (DeltaSeconds :type Float%20%28single-precision%29))
  (Variables|Default|SetCurrentStartLocation (Transformation|GetActorLocation))
  (for _index (range 0 5)
    (bind _output_get (Variables|Default|SetDiametr (* (Variables|Default|GetDiametr) 2.0)))
    (bind _output_get_2 (Variables|Default|SetCurrentStartLocation (+ (Variables|Default|GetCurrentStartLocation) (* (Transformation|GetActorForwardVector) (/ (Variables|Default|GetDiametr) 2.0)))))
    (Collision|SphereTraceByChannel _output_get_2 _output_get_2 (/ _output_get 2.0) "TraceTypeQuery1" false 0 "ForOneFrame"))
  (Variables|Default|SetCurrentStartLocation "0, 0, 0")
  (Variables|Default|SetDiametr 3e+01))

(fn ConstructionScript)