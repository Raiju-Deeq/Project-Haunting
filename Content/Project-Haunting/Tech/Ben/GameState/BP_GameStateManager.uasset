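; BP_GameStateManager tracks the current game state (main menu, running, paused or game over) and applies the matching pause and menu changes.
; BeginPlay creates the pause and game over widgets, and the construction script sets the starting state from a default.
; SetStateTo dispatches to per-state handlers that toggle game pause, print debug messages and show or remove those menus.
; The main menu handler is empty.
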(event Custom|RemovePauseMenu
  (if (Utilities|IsValid (Variables|Default|GetPauseMenu))
    (if (UserInterface|Viewport|IsinViewport (Variables|Default|GetPauseMenu))
      (Widget|RemovefromParent (Variables|Default|GetPauseMenu)))))

(event Custom|RemoveGameOverMenu
  (if (Utilities|IsValid (Variables|Default|GetGameOverMenu))
    (if (UserInterface|Viewport|IsinViewport (Variables|Default|GetGameOverMenu))
      (Widget|RemovefromParent (Variables|Default|GetGameOverMenu)))))

(event EventBeginPlay
  (bind _returnvalue (UserInterface|CreateWidget "/Game/Project-Haunting/Tech/Ben/GameState/UW_PauseMenu.UW_PauseMenu_C"))
  (Variables|Default|SetPauseMenu _returnvalue)
  (bind _returnvalue_2 (UserInterface|CreateWidget "/Game/Project-Haunting/Tech/Ben/GameState/UW_GameOver.UW_GameOver_C"))
  (Variables|Default|SetGameOverMenu _returnvalue_2))

(fn ConstructionScript
  (Variables|Default|SetCurrentGameState (Variables|Default|GetDefaultGameState)))

(fn SetStateto
  (params (NewState :type E_GameStates%20Enum :default "NewEnumerator0"))
  (bind _output_get (Variables|Default|SetCurrentGameState NewState))
  (switch Utilities|FlowControl|Switch|SwitchonE_GameStates _output_get
    (:NewEnumerator0
      (CallFunction|HandleMainMenu))
    (:NewEnumerator1
      (CallFunction|HandleGameRunning))
    (:NewEnumerator2
      (CallFunction|HandleGamePaused))
    (:NewEnumerator3
      (CallFunction|HandleGameOver))))

(fn GetCurrentState
  (return (Variables|Default|GetCurrentGameState)))

(fn HandleMainMenu)

(fn HandleGameRunning
  (Game|SetGamePaused false)
  (Development|PrintString "Game Is Now Runnning")
  (CallFunction|RemovePauseMenu)
  (CallFunction|RemoveGameOverMenu))

(fn HandleGamePaused
  (Game|SetGamePaused true)
  (Development|PrintString "Paused Game")
  (UserInterface|Viewport|AddtoViewport (Variables|Default|GetPauseMenu) 0))

(fn HandleGameOver
  (Game|SetGamePaused true)
  (Development|PrintString "Game Over")
  (UserInterface|Viewport|AddtoViewport (Variables|Default|GetGameOverMenu) 0))