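; BP_VerticalDoorDown is a door that slides along its local Z axis, downward by its name, when activated.
; Activate plays the DoorSlide timeline, whose DoorPosition track sets the Door component's relative Z location.
; Deactivate reverses the same timeline from its current position, and an Activated flag makes repeated calls to either event do nothing.
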(event EventActivate
  (if (not (Variables|Default|GetActivated))
    (Variables|Default|SetActivated true)
    (bind _doorposition (Timeline|DoorSlide Play)
      (:Update
        (Transformation|SetRelativeLocation (Variables|Default|GetDoor) (Math|Vector|MakeVector 0.0 0.0 _doorposition) false false)))))

(event EventDeactivate
  (if (Variables|Default|GetActivated)
    (Variables|Default|SetActivated false)
    (bind _doorposition (Timeline|DoorSlide Reverse)
      (:Update
        (Transformation|SetRelativeLocation (Variables|Default|GetDoor) (Math|Vector|MakeVector 0.0 0.0 _doorposition) false false)))))

(fn ConstructionScript)