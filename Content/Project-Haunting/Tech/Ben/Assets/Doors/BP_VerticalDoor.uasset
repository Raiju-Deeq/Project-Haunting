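; BP_VerticalDoor is a door that slides up or down on timelines, opened by player interaction or pressure plates.
; Interaction can require a named key from the player's found keys, unlocks first if locked, then toggles or auto-closes after a delay.
; Plates open it once enough are active, and releasing one closes it.
; At BeginPlay it collects rotate puzzles linked to it, but only prints their names.
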(event Custom|Close
  ;[0 0.01899 0.276] Open + Close Activation
  (if (Variables|Default|GetActivated)
    (Variables|Default|SetActivated false)
    (switch Utilities|FlowControl|Switch|SwitchonE_DoorAnimations (Variables|DoorConfig|GetAnimation)
      (:NewEnumerator0
        (Utilities|String|Reverse (Variables|Default|GetDoorSlideUp)))
      (:NewEnumerator1
        (Utilities|String|Reverse (Variables|Default|GetDoorSlideDown))))))

(event Custom|Open
  ;[0 0.01899 0.276] Open + Close Activation
  (if (not (Variables|Default|GetActivated))
    (Variables|Default|SetActivated true)
    (switch Utilities|FlowControl|Switch|SwitchonE_DoorAnimations (Variables|DoorConfig|GetAnimation)
      (:NewEnumerator0
        (Audio|Components|Audio|Play (Variables|Default|GetDoorSlideUp)))
      (:NewEnumerator1
        (Audio|Components|Audio|Play (Variables|Default|GetDoorSlideDown))))))

(event Custom|ProccesInteract
  (bind _openduration (Variables|DoorConfig|GetOpenDuration))
  ;[0 0.02178 0.2708] Process - Door Interact
  (Development|PrintString "Activated")
  (if (== _openduration 0.0)
    (if (Variables|Default|GetActivated)
      (CallFunction|Close)
      (else
        (CallFunction|Open)))
    (elif (not (Variables|Default|GetActivated))
      (CallFunction|Open)
      (Utilities|FlowControl|Delay _openduration)
      (CallFunction|Close))))

(event Custom|Unlock
  ;[0 0.05096 0.3958] Unlock Door
  (Variables|Default|SetLocked false)
  (Development|PrintString "Unlocked Door"))

(event EventInteract
  ;[0 0.01365 0.1927] Door Interact
  (if (Utilities|Enum|NotEqual(Enum) (Variables|DoorConfig|GetKeyName) "")
    (bind _asbp_first_person_character (Utilities|Casting|CastToBP_FirstPersonCharacter (Game|GetPlayerCharacter 0)))
    (if (Utilities|Array|ContainsItem (Variables|/Game/Dependency_Stuff/FirstPerson/Blueprints/BP_FirstPersonCharacter.BP_FirstPersonCharacter_C|GetFoundKeys _asbp_first_person_character) (Variables|DoorConfig|GetKeyName))
      (if (Variables|Default|GetLocked)
        (CallFunction|Unlock)
        (else
          (CallFunction|ProccesInteract)))
      (else
        (Development|PrintString "You Need To Find The Key")))
    (else
      (Variables|Default|SetLocked false)
      (if (Variables|Default|GetLocked)
        (CallFunction|Unlock)
        (else
          (CallFunction|ProccesInteract))))))

(event EventBeginPlay
  (bind _outactors (Actor|GetAllActorsOfClass "/Game/Project-Haunting/Tech/Ben/Assets/RotatingPuzzle/BP_RotatePuzzle.BP_RotatePuzzle_C"))
  (for _array_element _outactors
    (if (== (Variables|/Game/Project-Haunting/Tech/Ben/Assets/RotatingPuzzle/BP_RotatePuzzle.BP_RotatePuzzle_C|GetLinkedDoor _array_element) self)
      (Utilities|Array|AddUnique (Variables|Default|GetLinkedRotatorPuzzles) _array_element)))
  (Development|PrintString "Added Linked Puzzles")
  (for _array_element_2 (Variables|Default|GetLinkedRotatorPuzzles)
    (Development|PrintString (Utilities|GetDisplayName _array_element_2))))

(event EventActivate
  (params (Actor :type Actor%20Object%20Reference))
  ;[0 0.02398 0.2969] Pressure Plate / Puzzle - Activate + Deactivate
  (if (> (Variables|DoorConfig|GetPPR_Amount) 0)
    (Utilities|Array|AddUnique (Variables|Default|GetActivePressurePlates) Actor)
    (if (not (< (Utilities|Array|Length (Variables|Default|GetActivePressurePlates)) (Variables|DoorConfig|GetPPR_Amount)))
      (CallFunction|Open)
      (else
        (Development|PrintString "Not Enough Active Pressure Plates")))
    (else
      (Development|PrintString "Pressure Plates Do Not Activate This Door"))))

(event EventDeactivate
  (params (Actor :type Actor%20Object%20Reference))
  (bind _activepressureplates (Variables|Default|GetActivePressurePlates))
  ;[0 0.02398 0.2969] Pressure Plate / Puzzle - Activate + Deactivate
  (if (Utilities|Array|ContainsItem _activepressureplates Actor)
    (Utilities|Array|RemoveItem _activepressureplates Actor)
    (CallFunction|Close)))

(fn ConstructionScript)