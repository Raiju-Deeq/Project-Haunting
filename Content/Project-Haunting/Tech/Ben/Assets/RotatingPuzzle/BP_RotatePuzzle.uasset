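; Rotating puzzle actor that triggers a linked door when the player enters the correct left/right rotation sequence.
; Interact shows the puzzle widget and registers it as the character's active puzzle.
; Each input steps a wrapping index and plays a timeline lerping yaw along the shortest path, locking input until finished.
; At target length, input history is compared to the sequence; a wrong attempt clears it and closes the widget.
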(event Custom|HandleRotateLeft
  (Variables|Default|SetCurrentIndex (Math|Integer|%(Integer) (+ (Variables|Default|GetCurrentIndex) (- (Variables|Default|GetMaxRotationIndex) 1)) (Variables|Default|GetMaxRotationIndex))))

(event Custom|HandleRotateRight
  (Variables|Default|SetCurrentIndex (Math|Integer|%(Integer) (+ (Variables|Default|GetCurrentIndex) 1) (Variables|Default|GetMaxRotationIndex))))

(event Custom|RotateDirection
  (params (TargetDirection :type E_SpinDirection%20Enum :default "NewEnumerator0"))
  (bind _linkeddoor (Variables|PuzzleConfig|GetLinkedDoor))
  (Variables|Default|SetRecentInput TargetDirection)
  (if (not (Variables|Default|GetLocked))
    (switch Utilities|FlowControl|Switch|SwitchonE_SpinDirection TargetDirection
      (:NewEnumerator0
        (CallFunction|HandleRotateLeft))
      (:NewEnumerator1
        (CallFunction|HandleRotateRight)))
    (Variables|Default|SetNewAngle (* (Variables|Default|GetCurrentIndex) (Variables|Default|GetAngleRotation)))
    (CallFunction|AnimateAngle)
    (Utilities|Array|Add (Variables|Default|GetInputHistory) (Variables|Default|GetRecentInput))
    (if (>= (Utilities|Array|Length (Variables|Default|GetInputHistory)) (Utilities|Array|Length (Variables|PuzzleConfig|GetTargetSequence)))
      (if (Utilities|Array|Identical (Variables|Default|GetInputHistory) (Variables|PuzzleConfig|GetTargetSequence))
        (Development|PrintString "Correct Sequence")
        (Variables|Default|SetComplete true)
        (Utilities|IsValid _linkeddoor
          (:Is%20Valid
            (if (Utilities|DoesObjectImplementInterface _linkeddoor "/Game/Project-Haunting/Tech/Ben/Assets/BPI_Triggerable.BPI_Triggerable_C")
              (Class|BPITriggerable|Activate(Message) _linkeddoor self)
              (Utilities|Array|Clear (Variables|Default|GetInputHistory) :!label _label)
              (Widget|RemovefromParent (Variables|Default|GetPuzzleWidget)))))
        (else
          (Development|PrintString "Incorrect Sequence")
          (goto _label))))))

(event Custom|AnimateAngle
  (Variables|Default|SetLocked true)
  (Variables|Default|SetStartAngle (.Yaw (Math|Rotator|BreakRotator (Transformation|GetActorRotation))))
  (bind _rotation (Timeline|RotationAnim PlayFromStart)
    (:Update
      (Transformation|SetActorRotation (Math|Rotator|MakeRotator 0.0 0.0 (.yaw (Math|Rotator|Lerp(Rotator) (Math|Rotator|MakeRotator 0.0 0.0 (Variables|Default|GetStartAngle)) (Math|Rotator|MakeRotator 0.0 0.0 (Math|Conversions|ToFloat(Integer) (Variables|Default|GetNewAngle))) _rotation true)))))
    (:Finished
      (Variables|Default|SetLocked false))))

(event EventDeactivate
  (Development|PrintString "Deactivating Rotating Puzzle")
  (Widget|RemovefromParent (Variables|Default|GetPuzzleWidget)))

(event EventInteract
  ;[0 0.01365 0.1927] Rotating Puzzle Interact
  (Development|PrintString "Interacting With Rotating Puzzle")
  (UserInterface|Viewport|AddtoViewport (Variables|Default|GetPuzzleWidget) 0)
  (bind _asbp_first_person_character (Utilities|Casting|CastToBP_FirstPersonCharacter (Game|GetPlayerCharacter 0)))
  (Variables|/Game/Dependency_Stuff/FirstPerson/Blueprints/BP_FirstPersonCharacter.BP_FirstPersonCharacter_C|SetActiveRotatorPuzzle _asbp_first_person_character self))

(event EventBeginPlay
  ;[0 0.01365 0.1927] Rotating Puzzle Interact
  (bind _returnvalue (UserInterface|CreateWidget "/Game/Project-Haunting/Tech/Ben/Assets/RotatingPuzzle/W_RotatingPuzzle.W_RotatingPuzzle_C"))
  (Variables|Default|SetPuzzleWidget _returnvalue)
  (Variables|Default|SetMaxRotationIndex (Math|Float|Round (/ 3.6e+02 (Variables|Default|GetAngleRotation)))))

(fn ConstructionScript)